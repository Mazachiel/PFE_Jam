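; Choppable tree actor that falls when RobotCut fires, then regrows through young and old stages.
; Cutting swaps the full tree for a trunk, spins the actor to a random yaw, and tips the trunk over by timeline before hiding it.
; A timer starts regrowth: scale timelines grow the tree to young, making it cuttable again, then to old after RegrowTimeOld, updating Value at each stage.
; Older cut and regrowth logic remains disconnected.
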(event Custom|HideTrunk
  (params (NewParam :type Boolean))
  ;[1 1 1] HIDE TRUNK
  (Rendering|SetVisibility (Variables|Default|GetTree_trunk) false false))

(event Custom|RevealFullTree
  ;[1 1 1] REVEAL FULL TREE
  (Rendering|SetVisibility (Variables|Default|GetFullTree) true true))

(event Custom|Timber
  (CallFunction|RevealTrunk false)
  (Transformation|SetActorRotation (Math|Rotator|MakeRotator 0.0 0.0 (* 360 (Math|Random|RandomFloat))))
  (bind _floatcurvey (Timeline|Trunk%20Falling PlayFromStart)
    (:Update
      (Transformation|SetRelativeLocationAndRotation (Variables|Default|GetTree_trunk) "0,0.000000,160.000000" (Math|Rotator|Lerp(Rotator) "0,0.000000, 0" "95.000000, 0, 0" _floatcurvey) false false))
    (:Finished
      ;[1 1 1] TIMBER
      (Utilities|FlowControl|Delay 1.0)
      (CallFunction|HideTrunk false)
      (Utilities|Time|SetTimerbyEvent (delegate Custom|Regrowth) 2.0))))

(event Custom|Regrowth
  ;[1 1 1] REGROWTH
  (Transformation|SetRelativeScale3D (Variables|Default|GetFullTree) "0, 0, 0")
  (CallFunction|RevealFullTree)
  (bind _scalecurve (Timeline|toYoung_Timeline PlayFromStart)
    (:Update
      (Transformation|SetRelativeScale3D (Variables|Default|GetFullTree) _scalecurve))
    (:Finished
      (Variables|Default|SetValue 0.25)
      (Variables|Default|SetCut false)
      (Utilities|FlowControl|Delay (Variables|Default|GetRegrowTimeOld))
      (bind _scalecurve_tooold (Timeline|tooOld_Timeline PlayFromStart)
        (:Update
          (Transformation|SetRelativeScale3D (Variables|Default|GetFullTree) _scalecurve_tooold))
        (:Finished
          (Variables|Default|SetValue 0.75))))))

(event Custom|RobotCut
  ;[1 1 1] ROBOT CUT
  (if (not (Variables|Default|GetCut))
    (CallFunction|HideFullTree)
    (Variables|Default|SetCut true)
    (CallFunction|Timber)))

(event Custom|RevealTrunk
  (params (NewParam :type Boolean))
  ;[1 1 1] REVEAL TRUNK
  (Rendering|SetVisibility (Variables|Default|GetTree_trunk) true false))

(event Custom|HideFullTree
  ;[1 1 1] HIDE FULL TREE
  (Rendering|SetVisibility (Variables|Default|GetFullTree) false true))

(event EventBeginPlay)

(fn ConstructionScript)