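; Giant robot character that triggers the lifespan logic of other robots touching it and animates its size when it loses HP.
; Its Box overlap ignores itself, casts the other actor to Robot_Char, calls RobotLifespan on that robot's Robot_IA controller and prints the actor's name.
; OnHpLost restarts a timeline that uniformly rescales the static mesh as a multiple of its enlarged base scale.
; Tick and construction only call the parent.
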(event OnComponentBeginOverlap(Box)
  (params (OverlappedComponent :type Primitive%20Component%20Object%20Reference) (OtherActor :type Actor%20Object%20Reference) (OtherComp :type Primitive%20Component%20Object%20Reference) (OtherBodyIndex :type Integer) (bFromSweep :type Boolean) (SweepResult :type Hit%20Result%20Structure%20%28by%20ref%29))
  (if (!= OtherActor self)
    (bind _asrobot_char (Utilities|Casting|CastToRobot_Char OtherActor))
    (bind _asrobot_ia (Utilities|Casting|CastToRobot_IA (AI|GetAIController _asrobot_char)))
    (Default|RobotLifespan _asrobot_ia)
    (Development|PrintString (Utilities|GetDisplayName OtherActor))))

(event EventBeginPlay
  (|CallParentFunction) ; This node is disabled and will not be called.\nDrag off pins to build functionality.
)

(event Collision|EventActorBeginOverlap
  (params (OtherActor :type Actor%20Object%20Reference))
  (|CallParentFunction OtherActor) ; This node is disabled and will not be called.\nDrag off pins to build functionality.
)

(event EventTick
  (params (DeltaSeconds :type Float%20%28single-precision%29))
  (|CallParentFunction DeltaSeconds))

(event EventOnHpLost
  (bind _scale (Timeline|Timeline_1 PlayFromStart)
    (:Update
      (Transformation|SetRelativeScale3D (Variables|Default|GetStaticMesh) (Math|Vector|MakeVector (* 5.0 _scale) (* 5.0 _scale) (* 5.0 _scale))))))

(fn ConstructionScript
  (|CallParentFunction))