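; Robot character that displays floating text through a widget component and turns red at BeginPlay when flagged Infected.
; PlayTextInfoAnim shows supplied text and animates its height with a timeline before hiding it.
; A looping timer, with its interval randomized once at start, briefly shows widget-chosen text unless info text is playing.
; Tick rotates the widget to face the player's camera.
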(event Custom|ShowRandomText
  (bind _mrcirwin (Variables|Default|Getmrcirwin))
  ;[1 1 1] ShowText
  (if (not (Variables|Default|GetDisplayingTextInfo))
    (Default|SetText (Variables|Default|GetWidgetRef))
    (Rendering|SetVisibility _mrcirwin true false)
    (Utilities|FlowControl|Delay 2.0)
    (if (not (Variables|Default|GetDisplayingTextInfo))
      (Rendering|SetVisibility _mrcirwin false false))))

(event Custom|TriggerShowText
  (CallFunction|ShowRandomText))

(event Custom|PlayTextInfoAnim
  (params (TextToDisplay :type String))
  ;[1 1 1] Play Text Info
  (Rendering|Components|TextRender|SetText (Variables|/Game/StarterContent/Blueprints/Texttest.Texttest_C|GetTextBlock_55 (Variables|Default|GetWidgetRef)) (Utilities|Text|ToText(String) TextToDisplay))
  (Rendering|SetVisibility (Variables|Default|Getmrcirwin) true false)
  (Variables|Default|SetDisplayingTextInfo true)
  (Utilities|FlowControl|Delay 0.25)
  (bind _z_pos (Timeline|Timeline_0 PlayFromStart)
    (:Update
      (Transformation|SetRelativeLocation (Variables|Default|Getmrcirwin) (Math|Vector|MakeVector 0.0 0.0 (+ (Variables|Default|GetTextZOffset) _z_pos)) false false))
    (:Finished
      (Utilities|FlowControl|Delay 0.25)
      (Variables|Default|SetDisplayingTextInfo false)
      (Rendering|SetVisibility (Variables|Default|Getmrcirwin) false false))))

(event EventBeginPlay
  ;[1 1 1] GetWidgetRef
  (Variables|Default|SetTextZOffset (.z (Variables|/Script/Engine.SceneComponent|GetRelativeLocation (Variables|Default|Getmrcirwin))))
  (bind _astexttest (Utilities|Casting|CastToTexttest (UserInterface|GetUserWidgetObject (Variables|Default|Getmrcirwin))))
  (Variables|Default|SetWidgetRef _astexttest)
  (bind _output_get (Variables|Default|SetRandomTimer (Math|Random|RandomFloatinRange 1e+01 5e+01)))
  (Utilities|Time|SetTimerbyEvent (delegate Custom|TriggerShowText) _output_get true)
  (if (Variables|Default|GetInfected)
    (Rendering|Material|SetMaterial (Variables|Default|GetStaticMesh) 0 "/Game/Blueprints/red.red")))

(event Collision|EventActorBeginOverlap
  (params (OtherActor :type Actor%20Object%20Reference)))

(event EventTick
  (params (DeltaSeconds :type Float%20%28single-precision%29))
  ;[1 1 1] FaceCamera
  (bind _asplayer_blueprint (Utilities|Casting|CastToPlayer_Blueprint (Pawn|GetControlledPawn (Game|GetPlayerController 0))))
  (Transformation|SetWorldRotation (Variables|Default|Getmrcirwin) (Math|Rotator|FindLookatRotation (Transformation|GetWorldLocation (Variables|Default|Getmrcirwin)) (Transformation|GetWorldLocation (Variables|/Game/StarterContent/Blueprints/Player_Blueprint.Player_Blueprint_C|GetCamera _asplayer_blueprint))) false false))

(fn ConstructionScript)