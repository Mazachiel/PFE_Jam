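; AI controller for the big robot that runs the BT_IA_Robot behavior tree to react to trees it perceives.
; Perception updates from trees that are neither falling nor cut write the tree to the Target blackboard key and mirror the sensed state into CanSeeTree.
; The tree's location is projected onto the navmesh to set TargetDestination.
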(event OnTargetPerceptionUpdated(AIPerception)
  (params (Actor :type Actor%20Object%20Reference) (Stimulus :type AI%20Stimulus%20Structure))
  (bind _returnvalue (AI|GetBlackboard 0))
  (bind _astree_behavior (Utilities|Casting|CastToTreeBehavior Actor))
  (if (and (not (Variables|/Game/Clement/Blueprints/TreeBehavior.TreeBehavior_C|GetFalling _astree_behavior)) (not (Variables|/Game/Clement/Blueprints/TreeBehavior.TreeBehavior_C|GetCut _astree_behavior)))
    (AI|Components|Blackboard|SetValueasObject (AI|GetBlackboard 0) (Utilities|Name|MakeLiteralName "Target") _astree_behavior)
    (AI|Components|Blackboard|SetValueasVector _returnvalue (Utilities|Name|MakeLiteralName "TargetDestination") (.ProjectedLocation (AI|Navigation|ProjectPointtoNavigation (Transformation|GetActorLocation _astree_behavior) 0 0 "250.000000,250.000000,250.000000")))
    (AI|Components|Blackboard|SetValueasBool _returnvalue (Utilities|Name|MakeLiteralName "CanSeeTree") (.bSuccessfullySensed (Utilities|Struct|BreakAIStimulus Stimulus)))))

(event EventBeginPlay
  (AI|RunBehaviorTree "/Game/Blueprints/BT_IA_Robot.BT_IA_Robot")
  (Utilities|Casting|CastToBigRobot_Char (Pawn|GetControlledPawn)))

(event EventTick
  (params (DeltaSeconds :type Float%20%28single-precision%29)))

(fn ConstructionScript)