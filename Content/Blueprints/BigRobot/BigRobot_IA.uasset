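; AI controller for the BigRobot enemy that runs the BT_IA_BigRobot behavior tree on BeginPlay.
; AI perception updates are filtered to Robot_Char actors and written to the blackboard as Target, TargetDestination and CanSeeRobot.
; Target and location are written on both gained and lost sensing, while CanSeeRobot follows whether the stimulus was successfully sensed.
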(event OnTargetPerceptionUpdated(AIPerception)
  (params (Actor :type Actor%20Object%20Reference) (Stimulus :type AI%20Stimulus%20Structure))
  (bind _returnvalue (AI|GetBlackboard 0))
  (bind _asrobot_char (Utilities|Casting|CastToRobot_Char Actor))
  (AI|Components|Blackboard|SetValueasObject (AI|GetBlackboard 0) (Utilities|Name|MakeLiteralName "Target") _asrobot_char)
  (AI|Components|Blackboard|SetValueasVector _returnvalue (Utilities|Name|MakeLiteralName "TargetDestination") (Transformation|GetActorLocation _asrobot_char))
  (AI|Components|Blackboard|SetValueasBool _returnvalue (Utilities|Name|MakeLiteralName "CanSeeRobot") (.bSuccessfullySensed (Utilities|Struct|BreakAIStimulus Stimulus))))

(event EventBeginPlay
  (AI|RunBehaviorTree "/Game/Blueprints/BigRobot/BT_IA_BigRobot.BT_IA_BigRobot")
  (Utilities|Casting|CastToBigRobot_Char (Pawn|GetControlledPawn)))

(event EventTick
  (params (DeltaSeconds :type Float%20%28single-precision%29)))

(fn ConstructionScript)