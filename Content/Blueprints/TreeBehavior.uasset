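; Choppable tree actor that swaps to split top and bottom meshes when its collision box is first overlapped, then topples.
; The overlap hides the full mesh, shows both halves, sets Cut, and makes zeroed HMD base rotation/offset calls.
; Tick runs Timber, rotating the top each frame until an unnamed vector-parameter comparison passes.
; It then hides the top and sets IsFalling, which actually stops the rotation.
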(event OnComponentBeginOverlap(BoxCollision)
  (params (OverlappedComponent :type Primitive%20Component%20Object%20Reference) (OtherActor :type Actor%20Object%20Reference) (OtherComp :type Primitive%20Component%20Object%20Reference) (OtherBodyIndex :type Integer) (bFromSweep :type Boolean) (SweepResult :type Hit%20Result%20Structure%20%28by%20ref%29))
  (if (not (Variables|Default|GetCut))
    (CallFunction|HideFullTree)
    (CallFunction|SplitTree false)
    (Variables|Default|SetCut true)))

(event Custom|SplitTree
  (params (NewParam :type Boolean))
  (Rendering|SetVisibility (Variables|Default|GetTreeTopMesh) true false)
  (Class|OculusFunctionLibrary|SetBaseRotationandBaseOffsetinMeters "0, 0, 0" "0, 0, 0" "Orientation"))

(event Custom|HideFullTree
  (Rendering|SetVisibility (Variables|Default|GetTreeMesh) false false)
  (Class|OculusFunctionLibrary|SetBaseRotationandBaseOffsetinMeters "0, 0, 0" "0, 0, 0" "Orientation"))

(event Custom|Timber
  (if (Variables|Default|GetCut)
    (if (not (Variables|Default|GetIsFalling))
      (Transformation|AddRelativeRotation (Variables|Default|GetTreeTopMesh) "-1.000000, 0, 0" false false)
      (bind _returnvalue (Rendering|Material|GetVectorParameterValue 0 "None" :!class /Script/Engine.KismetMaterialLibrary))
      (if (Math|Vector|Equal(Vector) (Math|Conversions|ToVector(LinearColor) _returnvalue) (Variables|Default|GetVector3Rotation) -4e+01)
        (Rendering|SetVisibility (Variables|Default|GetTreeTopMesh) false false)
        (Variables|Default|SetIsFalling true)))))

(event EventBeginPlay)

(event Collision|EventActorBeginOverlap
  (params (OtherActor :type Actor%20Object%20Reference)))

(event EventTick
  (params (DeltaSeconds :type Float%20%28single-precision%29))
  (CallFunction|Timber))

(fn ConstructionScript)