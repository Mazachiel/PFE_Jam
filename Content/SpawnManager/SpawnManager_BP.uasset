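; Spawn manager that thins out level-placed trees and robots to a random subset, caching both sets on BeginPlay.
; UpdateSpawns shuffles each set and hides all but the first few, though RobotsToSpawn limits trees, TreesToSpawn limits robots, and each shows one fewer than requested.
; ClearUnspawned destroys hidden actors and calls LAUNCH on each visible robot's Robot_IA controller.
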(event Custom|UpdateSpawns
  (params (RobotsToSpawn :type Integer) (TreesToSpawn :type Integer))
  (bind _initiallyplacedtrees (Variables|Default|GetInitiallyPlacedTrees))
  (bind _initiallyplacedrobots (Variables|Default|GetInitiallyPlacedRobots))
  ;[1 1 1] Update Spawns
  (Utilities|Array|Shuffle _initiallyplacedtrees)
  (Utilities|Array|Shuffle (Variables|Default|GetInitiallyPlacedRobots))
  (for _index (range 0 (- (Utilities|Array|Length (Variables|Default|GetInitiallyPlacedTrees)) 1))
    (if (< _index (- RobotsToSpawn 1))
      (Rendering|SetActorHiddenInGame (Utilities|Array|Get(acopy) _initiallyplacedtrees _index) false)
      (else
        (Rendering|SetActorHiddenInGame (Utilities|Array|Get(acopy) _initiallyplacedtrees _index) true))))
  (for _index_2 (range 0 (- (Utilities|Array|Length _initiallyplacedrobots) 1))
    (if (< _index_2 (- TreesToSpawn 1))
      (Rendering|SetActorHiddenInGame (Utilities|Array|Get(acopy) _initiallyplacedrobots _index_2) false)
      (else
        (Rendering|SetActorHiddenInGame (Utilities|Array|Get(acopy) _initiallyplacedrobots _index_2) true)))))

(event Custom|ClearUnspawned
  (bind _actorstodestroyafterspawn (Variables|Default|GetActorsToDestroyAfterSpawn))
  (bind _actorstodestroyafterspawn_2 (Variables|Default|GetActorsToDestroyAfterSpawn))
  ;[1 1 1] Clear Unspawned
  (for _array_element (Variables|Default|GetInitiallyPlacedTrees)
    (if (Variables|/Script/Engine.Actor|GetbHidden _array_element)
      (Utilities|Array|Add _actorstodestroyafterspawn _array_element)))
  (for _array_element_2 (Variables|Default|GetInitiallyPlacedRobots)
    (if (Variables|/Script/Engine.Actor|GetbHidden _array_element_2)
      (Utilities|Array|Add _actorstodestroyafterspawn _array_element_2)
      (else
        (bind _asrobot_ia (Utilities|Casting|CastToRobot_IA (AI|GetAIController _array_element_2)))
        (Default|LAUNCH _asrobot_ia))))
  (Variables|Default|SetNumberOfActorsToDestroy (Utilities|Array|Length (Variables|Default|GetActorsToDestroyAfterSpawn)))
  (for _index (range 0 (- (Variables|Default|GetNumberOfActorsToDestroy) 1))
    (Actor|DestroyActor (Utilities|Array|Get(acopy) _actorstodestroyafterspawn_2 _index)))
  (Utilities|Array|Clear _actorstodestroyafterspawn_2))

(event EventBeginPlay
  (bind _outactors (Actor|GetAllActorsOfClass "/Game/Clement/Blueprints/TreeBehavior.TreeBehavior_C"))
  (bind _output_get (Variables|Default|SetInitiallyPlacedTrees _outactors))
  (bind _outactors_2 (Actor|GetAllActorsOfClass "/Game/Blueprints/Robot_Char.Robot_Char_C"))
  (bind _output_get_2 (Variables|Default|SetInitiallyPlacedRobots _outactors_2)))

(fn ConstructionScript)