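; Actor Blueprint that puts up the main menu and starts gameplay when Play is clicked.
; On BeginPlay it finds the level's SpawnManager_BP, creates the Main_Menu widget, hands it that manager and updates its slider maximum.
; The widget's Play button is bound to StartGame, which clears unspawned entries on the manager, enables shooting on the player pawn and adds the FastForward widget.
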(event Custom|StartGame
  (Default|ClearUnspawned (Variables|Default|GetNewVar_0))
  (bind _asplayer_blueprint (Utilities|Casting|CastToPlayer_Blueprint (Pawn|GetControlledPawn (Game|GetPlayerController 0))))
  (Variables|/Game/StarterContent/Blueprints/Player_Blueprint.Player_Blueprint_C|SetCanShoot _asplayer_blueprint true)
  (bind _returnvalue (UserInterface|CreateWidget "/Game/Erwan/UI/fastforward.FastForward_C"))
  (UserInterface|Viewport|AddtoViewport _returnvalue 0))

(event EventBeginPlay
  (bind _outactors (Actor|GetAllActorsOfClass "/Game/SpawnManager/SpawnManager_BP.SpawnManager_BP_C"))
  (bind _returnvalue (UserInterface|CreateWidget "/Game/Erwan/UI/Main_Menu.Main_Menu_C"))
  (bind _output_get (Variables|Default|SetUIref _returnvalue))
  (UserInterface|Viewport|AddtoViewport _output_get 0)
  (bind _output_get_2 (Variables|Default|SetNewVar_0 (Utilities|Array|Get(acopy) _outactors)))
  (Variables|/Game/Erwan/UI/Main_Menu.Main_Menu_C|SetSpawnManager _output_get _output_get_2)
  (Default|UpdateSliderMax (Variables|Default|GetUIref))
  (EventDispatchers|BindEventtoOnClicked (Variables|/Game/Erwan/UI/Main_Menu.Main_Menu_C|GetPlay (Variables|Default|GetUIref)) (delegate Custom|StartGame)))

(event EventTick
  (params (DeltaSeconds :type Float%20%28single-precision%29)))

(fn ConstructionScript)