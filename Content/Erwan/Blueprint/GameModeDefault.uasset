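; Default game mode that runs the main menu, level streaming and the start of play, and tracks living robots.
; On BeginPlay it shows the menu, hands it the SpawnManager and streams in the first map.
; Play clears unspawned entries, enables player shooting and adds the fast-forward and escape widgets.
; RobotAlive follows spawn and death events and is rebuilt when the SpawnManager finishes cleaning.
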(event Custom|StartGame
  (Default|ClearUnspawned (Variables|Default|GetSpawnManager))
  (bind _asplayer_blueprint (Utilities|Casting|CastToPlayer_Blueprint (Pawn|GetControlledPawn (Game|GetPlayerController 0))))
  (Variables|/Game/StarterContent/Blueprints/Player_Blueprint.Player_Blueprint_C|SetCanShoot _asplayer_blueprint true)
  (bind _returnvalue (UserInterface|CreateWidget "/Game/Erwan/UI/FastForward.FastForward_C"))
  (UserInterface|Viewport|AddtoViewport _returnvalue 0)
  (Input|SetInputModeGameandUI (Game|GetPlayerController 0) 0 "DoNotLock" true)
  (bind _returnvalue_2 (UserInterface|CreateWidget "/Game/Erwan/UI/EscapeMenu.EscapeMenu_C"))
  (UserInterface|Viewport|AddtoViewport _returnvalue_2 0))

(event Custom|LoadMap
  (params (NewMapIndex :type Integer) (LastMapIndex :type Integer))
  (bind _levels (Variables|Default|GetLevels))
  (bind _levels_2 (Variables|Default|GetLevels))
  (bind _returnvalue (Utilities|Array|Length _levels_2))
  (if (and (> LastMapIndex -1) (< LastMapIndex _returnvalue))
    (Game|UnloadStreamLevel(byName) (Utilities|Array|Get(acopy) _levels LastMapIndex) false))
  (if (and (> NewMapIndex -1) (< NewMapIndex _returnvalue))
    (Game|LoadStreamLevel(byName) (Utilities|Array|Get(acopy) _levels NewMapIndex) true)
    (Default|CallLoadedMap)))

(event Custom|SearchAllRobot
  (bind _outactors (Actor|GetAllActorsOfClass "/Game/Blueprints/Robot_Char.Robot_Char_C"))
  (Variables|Default|SetRobotAlive _outactors))

(event Custom|RobotDied
  (params (Robot :type Robot%20Char%20Object%20Reference))
  ;[1 1 1] Update RobotAlive
  (Utilities|Array|RemoveItem (Variables|Default|GetRobotAlive) Robot))

(event Custom|RobotSpawned
  (params (Robot :type Robot%20Char%20Object%20Reference))
  ;[1 1 1] Update RobotAlive
  (Utilities|Array|AddUnique (Variables|Default|GetRobotAlive) Robot))

(event EventBeginPlay
  (bind _outactors (Actor|GetAllActorsOfClass "/Game/SpawnManager/SpawnManager_BP.SpawnManager_BP_C"))
  (bind _returnvalue (UserInterface|CreateWidget "/Game/Erwan/UI/Main_Menu.Main_Menu_C"))
  (bind _output_get (Variables|Default|SetUIref _returnvalue))
  (UserInterface|Viewport|AddtoViewport _output_get 0)
  (Input|SetInputModeUIOnly (Game|GetPlayerController 0) _output_get "DoNotLock")
  (bind _output_get_2 (Variables|Default|SetSpawnManager (Utilities|Array|Get(acopy) _outactors)))
  (Variables|/Game/Erwan/UI/Main_Menu.Main_Menu_C|SetSpawnManager _output_get _output_get_2)
  (EventDispatchers|BindEventtoOnClicked (Variables|/Game/Erwan/UI/Main_Menu.Main_Menu_C|GetPlay (Variables|Default|GetUIref)) (delegate Custom|StartGame))
  (CallFunction|LoadMap 0 -1)
  (EventDispatchers|BindEventtoFinishedCleaning (Variables|Default|GetSpawnManager) (delegate Custom|SearchAllRobot)))

(fn ConstructionScript)